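; Mushroom actor for an SML2 game, apparently a power-up, that slides back and forth along the X axis.
; Tick moves it by a fixed step in the direction set by MoveLeft, so its speed depends on frame rate.
; Two box triggers set that flag when they overlap a StaticMeshActor, turning it around at obstacles.
; Destruction plays the power-up sound; pickup logic is not handled here.
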(event `self.ReceiveBeginPlay`)

(event `self.ReceiveTick`
  (params (DeltaSeconds :type "Float (single-precision)"))
  (bind (_returnvalue_x _returnvalue_y _returnvalue_z) (`KismetMathLibrary.BreakVector` (`self.K2_GetActorLocation`)))
  (bind (_returnvalue_x_2 _returnvalue_y_2 _returnvalue_z_2) (`KismetMathLibrary.BreakVector` (`self.K2_GetActorLocation`)))
  (if (`self.MoveLeft`)
    (`self.K2_SetActorLocation` (`KismetMathLibrary.MakeVector` (- _returnvalue_x_2 2.5) _returnvalue_y_2 _returnvalue_z_2))
    (else
      (`self.K2_SetActorLocation` (`KismetMathLibrary.MakeVector` (+ _returnvalue_x 2.5) _returnvalue_y _returnvalue_z)))))

(event `self.Box.OnComponentBeginOverlap`
  (params (OverlappedComponent :type "PrimitiveComponent Object Reference") (OtherActor :type "Actor Object Reference") (OtherComp :type "PrimitiveComponent Object Reference") (OtherBodyIndex :type Integer) (bFromSweep :type Boolean) (SweepResult :type "HitResult Structure (by ref)"))
  (cast `StaticMeshActor` OtherActor)
  (set `self.MoveLeft` false))

(event `self.Box1.OnComponentBeginOverlap`
  (params (OverlappedComponent :type "PrimitiveComponent Object Reference") (OtherActor :type "Actor Object Reference") (OtherComp :type "PrimitiveComponent Object Reference") (OtherBodyIndex :type Integer) (bFromSweep :type Boolean) (SweepResult :type "HitResult Structure (by ref)"))
  (cast `StaticMeshActor` OtherActor)
  (set `self.MoveLeft` true))

(event `self.ReceiveDestroyed`
  (`GameplayStatics.PlaySound2D` "/Game/SML2Game/sounds/Power_Up_-_SML2.Power_Up_-_SML2" 1.5 1.0 0.0 null null))

(fn `UserConstructionScript`)