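; fGoomba is an enemy that walks side to side while calling Jump every tick, and turns into a regular Goomba when hit.
; Two side boxes flip its direction on contact with static meshes, Goombas or Paper sprites.
; A third box calls Hit on a living Mario, while a capsule hit from Mario replaces it with a Goomba at its transform.
; A stomp sound plays when it is destroyed.
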(event `self.ReceiveBeginPlay`
  (`self.SetActorTickEnabled` false)
  (`KismetSystemLibrary.Delay` 0.5)
  (`self.SetActorTickEnabled` true))

(event `Hit`
  ;[1 1 1] Hit
  (`|SpawnActorFromClass` "/Game/SML2Game/blueprints/Goomba.Goomba_C" (`self.GetTransform`) "AlwaysSpawn" "OverrideRootScale" null null)
  (`self.K2_DestroyActor`))

(event `self.ReceiveTick`
  (params (DeltaSeconds :type "Float (single-precision)"))
  (bind (_returnvalue_x _returnvalue_y _returnvalue_z) (`KismetMathLibrary.BreakVector` (`self.K2_GetActorLocation`)))
  (bind (_returnvalue_x_2 _returnvalue_y_2 _returnvalue_z_2) (`KismetMathLibrary.BreakVector` (`self.K2_GetActorLocation`)))
  ;[1 1 1] Movement
  (if (`self.MoveLeft`)
    (`self.K2_SetActorLocation` (`KismetMathLibrary.MakeVector` (- _returnvalue_x_2 2.0) _returnvalue_y_2 _returnvalue_z_2))
    (else
      (`self.K2_SetActorLocation` (`KismetMathLibrary.MakeVector` (+ _returnvalue_x 2.0) _returnvalue_y _returnvalue_z))))
  (`self.Jump`))

(event `self.Box.OnComponentBeginOverlap`
  (params (OverlappedComponent :type "PrimitiveComponent Object Reference") (OtherActor :type "Actor Object Reference") (OtherComp :type "PrimitiveComponent Object Reference") (OtherBodyIndex :type Integer) (bFromSweep :type Boolean) (SweepResult :type "HitResult Structure (by ref)"))
  ;[1 1 1] Movement
  (cast `StaticMeshActor` OtherActor
    (:`then`
      (set `self.MoveLeft` false))
    (:`CastFailed`
      (cast `/Game/SML2Game/blueprints/Goomba` OtherActor
        (:`then`
          (set `self.MoveLeft` false))
        (:`CastFailed`
          (cast `PaperSpriteActor` OtherActor)
          (set `self.MoveLeft` false))))))

(event `self.Box1.OnComponentBeginOverlap`
  (params (OverlappedComponent :type "PrimitiveComponent Object Reference") (OtherActor :type "Actor Object Reference") (OtherComp :type "PrimitiveComponent Object Reference") (OtherBodyIndex :type Integer) (bFromSweep :type Boolean) (SweepResult :type "HitResult Structure (by ref)"))
  ;[1 1 1] Movement
  (cast `StaticMeshActor` OtherActor
    (:`then`
      (set `self.MoveLeft` true))
    (:`CastFailed`
      (cast `/Game/SML2Game/blueprints/Goomba` OtherActor
        (:`then`
          (set `self.MoveLeft` true))
        (:`CastFailed`
          (cast `PaperSpriteActor` OtherActor)
          (set `self.MoveLeft` true))))))

(event `self.Box3.OnComponentBeginOverlap`
  (params (OverlappedComponent :type "PrimitiveComponent Object Reference") (OtherActor :type "Actor Object Reference") (OtherComp :type "PrimitiveComponent Object Reference") (OtherBodyIndex :type Integer) (bFromSweep :type Boolean) (SweepResult :type "HitResult Structure (by ref)"))
  ;[1 1 1] Movement
  (bind _asbp_mario (cast `/Game/SML2Game/blueprints/bpMario` OtherActor))
  (if (not (`/Game/SML2Game/blueprints/bpMario.bisDead` _asbp_mario))
    (`/Game/SML2Game/blueprints/bpMario.Hit` _asbp_mario)
    (`self.SetActorTickEnabled` false)))

(event `self.CapsuleComponent.OnComponentHit`
  (params (HitComponent :type "PrimitiveComponent Object Reference") (OtherActor :type "Actor Object Reference") (OtherComp :type "PrimitiveComponent Object Reference") (NormalImpulse :type "Vector Structure") (Hit :type "HitResult Structure (by ref)"))
  ;[1 1 1] Movement
  (bind _asbp_mario (cast `/Game/SML2Game/blueprints/bpMario` OtherActor))
  (if (not (`/Game/SML2Game/blueprints/bpMario.bisDead` _asbp_mario))
    (`self.Hit`)
    (`self.SetActorTickEnabled` false)))

(event `self.ReceiveDestroyed`
  (`GameplayStatics.PlaySound2D` "/Game/SML2Game/sounds/Stomp_-_SML2.Stomp_-_SML2" 1.0 1.0 0.0 null null))

(fn `UserConstructionScript`)