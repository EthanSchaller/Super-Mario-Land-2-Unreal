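; Goomba enemy for an SML2 game that walks side to side, hurts Mario and can be killed by him.
; Tick moves it a fixed step and updates walk/fall flipbooks; two boxes set direction on non-Mario overlaps.
; A third box calls Mario's Hit, while a capsule hit from living Mario increments his kills and flags Dead.
; When Dead, it spawns GoombaDead and destroys itself, playing a stomp sound from Destroyed.
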(event `self.ReceiveBeginPlay`
  (`self.SetActorTickEnabled` false)
  (`KismetSystemLibrary.Delay` 0.3)
  (`self.SetActorTickEnabled` true))

(event `Change_Animations`
  (bind _goomba (`self.Goomba`))
  ;[1 1 1] Change animations
  (if (`self.Dead`)
    (`|SpawnActorFromClass` "/Game/SML2Game/blueprints/GoombaDead.GoombaDead_C" (`KismetMathLibrary.MakeTransform` (`SceneComponent.K2_GetComponentLocation` _goomba)) "AlwaysSpawn" "OverrideRootScale" null null)
    (`self.K2_DestroyActor`)
    (elif (`NavMovementComponent.IsFalling` (`self.CharacterMovement`))
      (`PaperFlipbookComponent.SetFlipbook` _goomba "/Game/SML2Game/sprites/sprtsExtra/goomba_fall.goomba_fall")
      (else
        (`PaperFlipbookComponent.SetFlipbook` _goomba "/Game/SML2Game/sprites/sprtsExtra/goomba_Walk.goomba_Walk")))))

(event `self.ReceiveTick`
  (params (DeltaSeconds :type "Float (single-precision)"))
  (bind (_returnvalue_x _returnvalue_y _returnvalue_z) (`KismetMathLibrary.BreakVector` (`self.K2_GetActorLocation`)))
  (bind (_returnvalue_x_2 _returnvalue_y_2 _returnvalue_z_2) (`KismetMathLibrary.BreakVector` (`self.K2_GetActorLocation`)))
  ;[1 1 1] Movement
  (`self.Change_Animations`)
  (if (`self.Dead`)
    _
    (elif (`self.MoveLeft`)
      (`self.K2_SetActorLocation` (`KismetMathLibrary.MakeVector` (- _returnvalue_x_2 2.0) _returnvalue_y_2 _returnvalue_z_2))
      (else
        (`self.K2_SetActorLocation` (`KismetMathLibrary.MakeVector` (+ _returnvalue_x 2.0) _returnvalue_y _returnvalue_z))))))

(event `self.Box.OnComponentBeginOverlap`
  (params (OverlappedComponent :type "PrimitiveComponent Object Reference") (OtherActor :type "Actor Object Reference") (OtherComp :type "PrimitiveComponent Object Reference") (OtherBodyIndex :type Integer) (bFromSweep :type Boolean) (SweepResult :type "HitResult Structure (by ref)"))
  ;[1 1 1] Movement
  (cast `/Game/SML2Game/blueprints/bpMario` OtherActor
    (:`CastFailed`
      (set `self.MoveLeft` false))))

(event `Hit`
  (params (NewParam :type "Actor Object Reference"))
  ;[1 1 1] Hit
  (bind _asbp_mario (cast `/Game/SML2Game/blueprints/bpMario` NewParam))
  (if (not (`/Game/SML2Game/blueprints/bpMario.bisDead` _asbp_mario))
    (bind _result (`/Engine/EditorBlueprintResources/StandardMacros.IncrementInt` (`/Game/SML2Game/blueprints/bpMario.iKills` _asbp_mario))
      (:`  `
        (set `/Game/SML2Game/blueprints/bpMario.iKills` _result _asbp_mario)
        (set `self.Dead` true)))))

(event `self.Box1.OnComponentBeginOverlap`
  (params (OverlappedComponent :type "PrimitiveComponent Object Reference") (OtherActor :type "Actor Object Reference") (OtherComp :type "PrimitiveComponent Object Reference") (OtherBodyIndex :type Integer) (bFromSweep :type Boolean) (SweepResult :type "HitResult Structure (by ref)"))
  ;[1 1 1] Movement
  (cast `/Game/SML2Game/blueprints/bpMario` OtherActor
    (:`CastFailed`
      (set `self.MoveLeft` true))))

(event `self.Box3.OnComponentBeginOverlap`
  (params (OverlappedComponent :type "PrimitiveComponent Object Reference") (OtherActor :type "Actor Object Reference") (OtherComp :type "PrimitiveComponent Object Reference") (OtherBodyIndex :type Integer) (bFromSweep :type Boolean) (SweepResult :type "HitResult Structure (by ref)"))
  ;[1 1 1] Movement
  (bind _asbp_mario (cast `/Game/SML2Game/blueprints/bpMario` OtherActor))
  (if (not (`self.Dead`))
    (`/Game/SML2Game/blueprints/bpMario.Hit` _asbp_mario)
    (if (`/Game/SML2Game/blueprints/bpMario.bisDead` _asbp_mario)
      (`self.SetActorTickEnabled` false))))

(event `self.CapsuleComponent.OnComponentHit`
  (params (HitComponent :type "PrimitiveComponent Object Reference") (OtherActor :type "Actor Object Reference") (OtherComp :type "PrimitiveComponent Object Reference") (NormalImpulse :type "Vector Structure") (Hit :type "HitResult Structure (by ref)"))
  ;[1 1 1] Movement
  (`self.Hit` OtherActor))

(event `self.ReceiveDestroyed`
  (`GameplayStatics.PlaySound2D` "/Game/SML2Game/sounds/Stomp_-_SML2.Stomp_-_SML2" 1.0 1.0 0.0 null null))

(fn `UserConstructionScript`)