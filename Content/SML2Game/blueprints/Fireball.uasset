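; Mario's fireball projectile, a bouncing pawn that plays a sound on spawn and destroys itself after five seconds.
; Each tick it steps left or right and calls Jump, while two side boxes flip its direction on overlap with anything but Mario or fireballs.
; Capsule hits and overlaps destroy fBlocks and Goombas or call Hit on fGoombas, remove the fireball, and increment Mario's kill count for enemies.
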(event `self.ReceiveBeginPlay`
  (`GameplayStatics.PlaySound2D` "/Game/SML2Game/sounds/Fireball_-_SML2.Fireball_-_SML2" 1.0 1.0 0.0 null null)
  (`KismetSystemLibrary.Delay` 5.0)
  (`self.K2_DestroyActor`))

(event `Hit_Enemy`
  ;[1 1 1] Hit an Enemy
  (bind _asbp_mario (cast `/Game/SML2Game/blueprints/bpMario` (`GameplayStatics.GetPlayerPawn` 0)))
  (bind _result (`/Engine/EditorBlueprintResources/StandardMacros.IncrementInt` (`/Game/SML2Game/blueprints/bpMario.iKills` _asbp_mario))
    (:`  `
      (set `/Game/SML2Game/blueprints/bpMario.iKills` _result _asbp_mario))))

(event `self.ReceiveTick`
  (params (DeltaSeconds :type "Float (single-precision)"))
  (bind (_returnvalue_x _returnvalue_y _returnvalue_z) (`KismetMathLibrary.BreakVector` (`self.K2_GetActorLocation`)))
  (bind (_returnvalue_x_2 _returnvalue_y_2 _returnvalue_z_2) (`KismetMathLibrary.BreakVector` (`self.K2_GetActorLocation`)))
  ;[1 1 1] movement
  (if (`self.MoveRight`)
    (`self.K2_SetActorLocation` (`KismetMathLibrary.MakeVector` (+ _returnvalue_x_2 7.5) _returnvalue_y_2 _returnvalue_z_2))
    (else
      (`self.K2_SetActorLocation` (`KismetMathLibrary.MakeVector` (- _returnvalue_x 7.5) _returnvalue_y _returnvalue_z))))
  (`self.Jump`))

(event `self.CapsuleComponent.OnComponentHit`
  (params (HitComponent :type "PrimitiveComponent Object Reference") (OtherActor :type "Actor Object Reference") (OtherComp :type "PrimitiveComponent Object Reference") (NormalImpulse :type "Vector Structure") (Hit :type "HitResult Structure (by ref)"))
  ;[1 1 1] Collision
  (bind _asf_block (cast `/Game/SML2Game/blueprints/fBlock` OtherActor)
    (:`then`
      (`self.K2_DestroyActor` _asf_block)
      (`self.K2_DestroyActor`))
    (:`CastFailed`
      (bind _asgoomba (cast `/Game/SML2Game/blueprints/Goomba` OtherActor)
        (:`then`
          (`self.Hit_Enemy`)
          (`self.K2_DestroyActor` _asgoomba)
          (`self.K2_DestroyActor`))
        (:`CastFailed`
          (bind _asf_goomba (cast `/Game/SML2Game/blueprints/fGoomba` OtherActor))
          (`self.Hit_Enemy`)
          (`/Game/SML2Game/blueprints/fGoomba.Hit` _asf_goomba)
          (`self.K2_DestroyActor`))))))

(event `self.CapsuleComponent.OnComponentBeginOverlap`
  (params (OverlappedComponent :type "PrimitiveComponent Object Reference") (OtherActor :type "Actor Object Reference") (OtherComp :type "PrimitiveComponent Object Reference") (OtherBodyIndex :type Integer) (bFromSweep :type Boolean) (SweepResult :type "HitResult Structure (by ref)"))
  ;[1 1 1] Collision
  (bind _asf_block (cast `/Game/SML2Game/blueprints/fBlock` OtherActor)
    (:`then`
      (`self.K2_DestroyActor` _asf_block)
      (`self.K2_DestroyActor`))
    (:`CastFailed`
      (bind _asgoomba (cast `/Game/SML2Game/blueprints/Goomba` OtherActor)
        (:`then`
          (`self.Hit_Enemy`)
          (`self.K2_DestroyActor` _asgoomba)
          (`self.K2_DestroyActor`))
        (:`CastFailed`
          (bind _asf_goomba (cast `/Game/SML2Game/blueprints/fGoomba` OtherActor))
          (`self.Hit_Enemy`)
          (`/Game/SML2Game/blueprints/fGoomba.Hit` _asf_goomba)
          (`self.K2_DestroyActor`))))))

(event `self.Box.OnComponentBeginOverlap`
  (params (OverlappedComponent :type "PrimitiveComponent Object Reference") (OtherActor :type "Actor Object Reference") (OtherComp :type "PrimitiveComponent Object Reference") (OtherBodyIndex :type Integer) (bFromSweep :type Boolean) (SweepResult :type "HitResult Structure (by ref)"))
  ;[1 1 1] Collision
  (cast `/Game/SML2Game/blueprints/bpMario` OtherActor
    (:`CastFailed`
      (cast `/Game/SML2Game/blueprints/Fireball` OtherActor
        (:`CastFailed`
          (set `self.MoveRight` true))))))

(event `self.Box1.OnComponentBeginOverlap`
  (params (OverlappedComponent :type "PrimitiveComponent Object Reference") (OtherActor :type "Actor Object Reference") (OtherComp :type "PrimitiveComponent Object Reference") (OtherBodyIndex :type Integer) (bFromSweep :type Boolean) (SweepResult :type "HitResult Structure (by ref)"))
  ;[1 1 1] Collision
  (cast `/Game/SML2Game/blueprints/bpMario` OtherActor
    (:`CastFailed`
      (cast `/Game/SML2Game/blueprints/Fireball` OtherActor
        (:`CastFailed`
          (set `self.MoveRight` false))))))

(fn `UserConstructionScript`)